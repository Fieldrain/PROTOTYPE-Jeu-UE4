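; Player Character Blueprint that handles movement, look, jump, crouch, sprint and throwing a disc.
; BeginPlay spawns a Projectile_BP, snaps it to the left-hand socket and has the capsule ignore it when moving.
; Tir detaches that same disc and activates its projectile and rotating movement components.
; Crouch supports hold and toggle inputs, sprint switches walk speed, and P opens a cached pause widget and pauses the game.
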(event Custom|Set%20Running
  (params (Is%20Running :type Boolean))
  (bind _charactermovement (Variables|Character|GetCharacterMovement))
  ;[1 1 1] Sprint Shift
  (Variables|Input|SetIsRunning Is%20Running)
  (if Is%20Running
    (Variables|/Script/Engine.CharacterMovementComponent|SetMaxWalkSpeed _charactermovement 6e+02)
    (else
      (Variables|/Script/Engine.CharacterMovementComponent|SetMaxWalkSpeed _charactermovement 3e+02))))

(event Custom|Tir
  (bind _disque (Variables|Components|GetDisque))
  ;[1 1 1] Tir
  (Class|SceneComponent|DetachfromParent (Variables|/Game/Projectile/Blueprint/Projectile_BP.Projectile_BP_C|GetMesh (Variables|Components|GetDisque)) true true)
  (Components|Activation|Activate (Variables|/Game/Projectile/Blueprint/Projectile_BP.Projectile_BP_C|GetProjectileMovement _disque) false)
  (Components|Activation|Activate (Variables|/Game/Projectile/Blueprint/Projectile_BP.Projectile_BP_C|GetRotatingMovement _disque) false))

(event EventBeginPlay
  ;[1 1 1] HUD of Character
  (CallFunction|SetupPerso))

(event Collision|EventActorBeginOverlap
  (params (OtherActor :type Actor%20Object%20Reference)))

(event EventTick
  (params (DeltaSeconds :type Float%20%28single-precision%29)))

(event Input|ActionEvents|InputActionSaut
  ;[1 1 1] Saut
  (:Pressed
    (Character|Jump)))

(event Input|ActionEvents|InputActionAccroupiContinue
  ;[1 1 1] Accroupi C/CRTL
  (:Pressed
    (if (AI|Components|NavMovement|IsCrouching (Variables|Character|GetCharacterMovement))
      (Character|UnCrouch)
      (else
        (Character|Crouch)))))

(event Input|ActionEvents|InputActionAccroupiMaintenu
  ;[1 1 1] Accroupi C/CRTL
  (:Pressed
    (if (AI|Components|NavMovement|IsCrouching (Variables|Character|GetCharacterMovement))
      (Character|UnCrouch :!label _label)
      (else
        (Character|Crouch))))
  (:Released
    (goto _label)))

(event Input|ActionEvents|InputActionSprintMaintenu
  ;[1 1 1] Sprint Shift
  (:Pressed
    (CallFunction|SetRunning true))
  (:Released
    (CallFunction|SetRunning false)))

(event Input|ActionEvents|InputActionTir
  ;[1 1 1] Tir
  (:Pressed
    (CallFunction|Tir)))

(event Input|AxisEvents|InputAxisDeplacementHorizontal
  (params (AxisValue :type Float%20%28single-precision%29))
  ;[1 1 1] Deplacement D/Q
  (Pawn|Input|AddMovementInput (Math|Vector|GetRightVector (Class|KismetMathLibrary|MakeRot 0.0 (.Yaw (Class|KismetMathLibrary|BreakRot (Pawn|GetControlRotation :!class /Script/Engine.Pawn))) 0.0)) AxisValue false))

(event Input|AxisEvents|InputAxisRegardVertical
  (params (AxisValue :type Float%20%28single-precision%29))
  ;[1 1 1] Regard
  (Pawn|Input|AddControllerPitchInput AxisValue))

(event Input|AxisEvents|InputAxisDeplacementVertical
  (params (AxisValue :type Float%20%28single-precision%29))
  ;[1 1 1] Deplacement Z/S
  (Pawn|Input|AddMovementInput (Math|Vector|GetForwardVector (Class|KismetMathLibrary|MakeRot 0.0 (.Yaw (Class|KismetMathLibrary|BreakRot (Pawn|GetControlRotation :!class /Script/Engine.Pawn))) 0.0)) AxisValue false))

(event Input|AxisEvents|InputAxisRegardHorizontal
  (params (AxisValue :type Float%20%28single-precision%29))
  ;[1 1 1] Regard
  (Pawn|Input|AddControllerYawInput AxisValue))

(event Input|KeyboardEvents|P
  ;[1 1 1] PauseMenu
  (:Pressed
    (Utilities|IsValid (Variables|Default|GetPauseMenuptr)
      (:Is%20Valid
        _)
      (:Is%20Not%20Valid
        (bind _returnvalue (UserInterface|CreateWidget "/Game/Widget/Pause_Game.Pause_Game_C"))
        (Variables|Default|SetPauseMenuptr _returnvalue)))
    (Input|SetInputModeUIOnly (Game|GetPlayerController 0) (Variables|Default|GetPauseMenuptr) false)
    (UserInterface|Viewport|AddtoViewport (Variables|Default|GetPauseMenuptr) 0)
    (Game|SetGamePaused true)))

(fn ConstructionScript)

(fn SetupPerso
  (bind _returnvalue (Game|SpawnActorfromClass "/Game/Projectile/Blueprint/Projectile_BP.Projectile_BP_C" (Transformation|GetActorTransform) true 0 0))
  (bind _output_get (Variables|Components|SetDisque _returnvalue))
  (Collision|IgnoreActorwhenMoving (Variables|Collision|GetCapsuleComponent) _output_get true)
  (Class|SceneComponent|Attachto (Variables|/Game/Projectile/Blueprint/Projectile_BP.Projectile_BP_C|GetMesh (Variables|Components|GetDisque)) (Variables|Character|GetMesh) "hand_l" "SnapToTargetIncludingScale" true))