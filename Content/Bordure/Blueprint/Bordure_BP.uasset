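; Bordure_BP is an electric-fence-style border: two posts joined by three beam particle arcs, with a collision box that launches characters hitting it.
; The construction script spaces the posts by Ecart, scales them in height and fits the box between them using Ecart and Hauteur.
; BeginPlay sets beam endpoints at top, middle and bottom.
; Launch velocity follows the character mesh's relative-rotation forward vector, at max speed plus ForceRepulsion.
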(event OnComponentHit(Box)
  (params (OtherActor :type Actor%20Object%20Reference) (OtherComp :type Primitive%20Component%20Object%20Reference) (NormalImpulse :type Vector) (Hit :type Hit%20Result%20Structure%20%28by%20ref%29))
  (bind _ascharacter_bp (Utilities|Casting|CastToCharacter_BP OtherActor))
  (Character|LaunchCharacter _ascharacter_bp (* (Math|Vector|GetForwardVector (Variables|/Script/Engine.SceneComponent|GetRelativeRotation (Variables|/Script/Engine.Character|GetMesh _ascharacter_bp))) (+ (Class|MovementComponent|GetMaxSpeed (Variables|/Script/Engine.Character|GetCharacterMovement _ascharacter_bp)) (Variables|Default|GetForceRepulsion))) false false))

(event EventBeginPlay
  (bind _hauteur (Variables|Default|GetHauteur))
  (bind _borddroit (Variables|Default|GetBordDroit))
  (bind _bordgauche (Variables|Default|GetBordGauche))
  (bind _returnvalue (Transformation|GetWorldLocation _bordgauche))
  (bind _returnvalue_2 (Transformation|GetWorldLocation _borddroit))
  (CallFunction|SetArc _returnvalue _returnvalue_2 (- _hauteur 5e+01) (Variables|Default|GetHaut))
  (CallFunction|SetArc _returnvalue _returnvalue_2 (/ _hauteur 2.0) (Variables|Default|GetMilieu))
  (CallFunction|SetArc _returnvalue _returnvalue_2 5e+01 (Variables|Default|GetBas)))

(event Collision|EventActorBeginOverlap
  (params (OtherActor :type Actor%20Object%20Reference)))

(event EventTick
  (params (DeltaSeconds :type Float%20%28single-precision%29)))

(fn ConstructionScript
  (bind _returnvalue (|(({C030C698-4266-7249-5FBD-40B43B86A27F}*1)/500)))
  (bind _borddroit (Variables|Default|GetBordDroit))
  (bind _bordgauche (Variables|Default|GetBordGauche))
  (bind _ecart (Variables|Default|GetEcart))
  (bind _returnvalue_2 (/ _ecart 2.0))
  (bind _returnvalue_3 (Math|Vector|MakeVector 1.0 1.0 _returnvalue))
  (CallFunction|SetBord _borddroit (* _returnvalue_2 -1.0) (Variables|/Script/Engine.SceneComponent|GetRelativeLocation _borddroit) _returnvalue_3)
  (CallFunction|SetBord _bordgauche _returnvalue_2 (Variables|/Script/Engine.SceneComponent|GetRelativeLocation _bordgauche) _returnvalue_3)
  (CallFunction|SetBox))

(fn SetArc
  (params (LocationDebut :type Vector) (Location%20Fin :type Vector) (Emplacement :type Float%20%28single-precision%29) (Particle :type Particle%20System%20Component%20Object%20Reference))
  (bind (_x _y _z) (Math|Vector|BreakVector LocationDebut))
  (bind (_x_2 _y_2 _z_2) (Math|Vector|BreakVector Location%20Fin))
  (Components|Activation|Activate Particle false)
  (Class|ParticleSystemComponent|SetBeamSourcePoint Particle 0 (Math|Vector|MakeVector _x _y (+ _z Emplacement)))
  (Class|ParticleSystemComponent|SetBeamTargetPoint Particle 0 (Math|Vector|MakeVector _x_2 _y_2 (+ Emplacement _z_2))))

(fn SetBord
  (params (Bord :type Static%20Mesh%20Component%20Object%20Reference) (Ecart :type Float%20%28single-precision%29) (Location :type Vector) (Scale :type Vector))
  (bind (_x _y _z) (Math|Vector|BreakVector Location))
  (Transformation|SetRelativeScale3D Bord Scale)
  (Transformation|SetRelativeLocation Bord (Math|Vector|MakeVector _x (+ _y Ecart) _z) true))

(fn SetBox
  (bind _box (Variables|Default|GetBox))
  (bind _hauteur (Variables|Default|GetHauteur))
  (bind _returnvalue (/ _hauteur 2.0))
  (bind _relativelocation (Variables|/Script/Engine.SceneComponent|GetRelativeLocation _box))
  (bind (_x _y _z) (Math|Vector|BreakVector _relativelocation))
  (Components|Box|SetBoxExtent _box (Math|Vector|MakeVector 25.0 (/ (- (Variables|Default|GetEcart) 5e+01) 2.0) _returnvalue) true)
  (Transformation|SetRelativeLocation _box (Math|Vector|MakeVector _x _y (+ _z _returnvalue)) true))