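; Platform actor with a destructible mesh that restores itself after a period of inactivity.
; While IsActive is false, Tick accumulates a timer up to TempsInactif, then reapplies the mesh and reactivates the platform; deactivation happens outside these graphs.
; ChangeMesh finds the GestMesh.ListMesh entry whose object name matches the MeshName enum string, and also runs in the construction script to set the initial mesh.
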(event EventBeginPlay)

(event Collision|EventActorBeginOverlap
  (params (OtherActor :type Actor%20Object%20Reference)))

(event EventTick
  (params (DeltaSeconds :type Float%20%28single-precision%29))
  (if (not (Variables|Plateforme|GetIsActive))
    (if (< (Variables|Default|GetTimer) (Variables|Plateforme|GetTempsInactif))
      (Variables|Default|SetTimer (+ (Variables|Default|GetTimer) DeltaSeconds))
      (else
        (CallFunction|ChangeMesh (Utilities|String|EnumtoString (.MeshName (Utilities|Struct|BreakGestionMesh (Variables|Plateforme|GetGestMesh)))))
        (Variables|Default|SetTimer 0.0)
        (Variables|Plateforme|SetIsActive true)))))

(fn ConstructionScript
  (CallFunction|ChangeMesh (Utilities|String|EnumtoString (.MeshName (Utilities|Struct|BreakGestionMesh (Variables|Plateforme|GetGestMesh))))))

(fn ChangeMesh
  (params (MeshName :type String))
  (bind _array_element (Utilities|Array|ForEachLoopwithBreak (.ListMesh (Utilities|Struct|BreakGestionMesh (Variables|Plateforme|GetGestMesh))) :!label _label)
    (:LoopBody
      (if (Utilities|Enum|Equal(Enum) (Utilities|GetObjectName _array_element) MeshName)
        (Class|DestructibleComponent|SetDestructibleMesh (Variables|Default|GetMesh) _array_element)
        (goto _label Break)))))